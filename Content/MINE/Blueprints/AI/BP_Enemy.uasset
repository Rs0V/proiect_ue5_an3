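; BP_Enemy is a melee enemy that damages the player on contact and carries a spotlight that reacts to the player's proximity.
; Each Tick, the clamped, normalized distance to the player drives the spotlight's cone angles and its color, blended per channel by LerpColor.
; Hitting BP_Player applies random melee damage and plays a punch sound.
; A multiplier zeroed until a timer resets it provides the cooldown, though sound still plays on every hit.
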(event Custom|ResetDamageMultiplier
  (Variables|Default|SetdamageMultiplier 1))

(event EventBeginPlay)

(event EventTick
  (params (DeltaSeconds :type Float%20%28single-precision%29))
  (bind _returnvalue (Game|GetPlayerCharacter 0))
  (bind _returnvalue_2 (Transformation|GetActorLocation))
  (bind _disttoplayerrange (Variables|Default|GetdistToPlayerRange))
  (bind _innerconeanglerange (Variables|Default|GetinnerConeAngleRange))
  (bind _outerconeanglerange (Variables|Default|GetouterConeAngleRange))
  (bind _returnvalue_3 (Transformation|GetActorLocation _returnvalue))
  (bind _returnvalue_4 (- (.value (.upperbound _disttoplayerrange)) (.value (.lowerbound _disttoplayerrange))))
  (bind _returnvalue_5 (Math|Vector|Distance(Vector) _returnvalue_3 _returnvalue_2))
  (bind _returnvalue_6 (- _returnvalue_5 (.value (.lowerbound _disttoplayerrange))))
  (bind _returnvalue_7 (/ _returnvalue_6 _returnvalue_4))
  (bind _returnvalue_8 (Math|Float|Clamp(Float) _returnvalue_7))
  (Rendering|Lighting|SetInnerConeAngle (Variables|Default|GetSpotLight) (Math|Float|Lerp (.value (.lowerbound _innerconeanglerange)) (.value (.upperbound _innerconeanglerange)) _returnvalue_8))
  (Rendering|Lighting|SetOuterConeAngle (Variables|Default|GetSpotLight) (Math|Float|Lerp (.value (.lowerbound _outerconeanglerange)) (.value (.upperbound _outerconeanglerange)) _returnvalue_8))
  (Rendering|Components|Light|SetLightColor (Variables|Default|GetSpotLight) (Math|Conversions|ToLinearColor(Color) (CallFunction|LerpColor (Variables|Default|GetcloseColor) (Variables|Default|GetfarColor) _returnvalue_8)) true))

(event Collision|EventHit
  (params (MyComp :type Primitive%20Component%20Object%20Reference) (Other :type Actor%20Object%20Reference) (OtherComp :type Primitive%20Component%20Object%20Reference) (bSelfMoved :type Boolean) (HitLocation :type Vector :default "0, 0, 0") (HitNormal :type Vector :default "0, 0, 0") (NormalImpulse :type Vector :default "0, 0, 0") (Hit :type Hit%20Result%20Structure%20%28by%20ref%29))
  (bind _damagerange (Variables|Default|GetdamageRange))
  (bind _asbp_player (Utilities|Casting|CastToBP_Player Other))
  (Game|Damage|ApplyDamage _asbp_player (Math|Conversions|ToFloat(Integer) (* (Variables|Default|GetdamageMultiplier) (Math|Random|RandomIntegerinRange (.value (.lowerbound _damagerange)) (.value (.upperbound _damagerange))))) (Pawn|GetController) self "/Game/MINE/Blueprints/AI/BP_MeleeDamage.BP_MeleeDamage_C")
  (Audio|PlaySoundatLocation "/Game/MINE/Maps/MainMenu/Sounds/punch_sound.punch_sound" (Transformation|GetActorLocation) "0, 0, 0" 1.0 1.0 0.0 0 0 0 0)
  (if (!= (Variables|Default|GetdamageMultiplier) 0)
    (Variables|Default|SetdamageMultiplier 0)
    (Utilities|Time|SetTimerbyEvent (delegate Custom|ResetDamageMultiplier) (Variables|Default|GetdamageCooldownTime))))

(fn ConstructionScript)

(fn LerpColor
  (params (a :type Color%20Structure) (b :type Color%20Structure) (alpha :type Float%20%28double-precision%29))
  (bind (_b _g _r _a) (Math|Color|BreakColor a))
  (bind (_b_2 _g_2 _r_2 _a_2) (Math|Color|BreakColor b))
  (return (Math|Color|MakeColor (Math|Conversions|ToByte(Integer) (Class|KismetMathLibrary|Round64 (Math|Float|Lerp (Math|Conversions|ToFloat(Byte) _b) (Math|Conversions|ToFloat(Byte) _b_2) alpha))) (Math|Conversions|ToByte(Integer) (Class|KismetMathLibrary|Round64 (Math|Float|Lerp (Math|Conversions|ToFloat(Byte) _g) (Math|Conversions|ToFloat(Byte) _g_2) alpha))) (Math|Conversions|ToByte(Integer) (Class|KismetMathLibrary|Round64 (Math|Float|Lerp (Math|Conversions|ToFloat(Byte) _r) (Math|Conversions|ToFloat(Byte) _r_2) alpha))) (Math|Conversions|ToByte(Integer) (Class|KismetMathLibrary|Round64 (Math|Float|Lerp (Math|Conversions|ToFloat(Byte) _a) (Math|Conversions|ToFloat(Byte) _a_2) alpha))))))