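; Enemy AI controller that runs BT_Enemy and tracks the player by sight.
; On BeginPlay it starts the behavior tree, then AI Perception updates feed HandleSight, which ignores non-sight senses and actors other than the player character.
; HandleSight sets the targetActor blackboard key to the player while seen and clears it when sight is lost, also storing the stimulus location as lastKnownLocation.
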(event OnTargetPerceptionUpdated(AIPerception)
  (params (Actor :type Actor%20Object%20Reference) (Stimulus :type AI%20Stimulus%20Structure))
  (CallFunction|HandleSight Actor Stimulus))

(event EventBeginPlay
  (AI|RunBehaviorTree "/Game/MINE/Blueprints/AI/BT_Enemy.BT_Enemy"))

(event EventTick
  (params (DeltaSeconds :type Float%20%28single-precision%29)))

(fn ConstructionScript)

(fn HandleSight
  (params (actor :type Actor%20Object%20Reference) (stimulus :type AI%20Stimulus%20Structure))
  (bind _returnvalue (Class|AIPerceptionSystem|GetSenseClassforStimulus stimulus))
  (if (== _returnvalue "/Script/AIModule.AISense_Sight")
    (if (== (LocalVariables|GetActor) (Game|GetPlayerCharacter 0))
      (AI|Components|Blackboard|SetValueasObject (Variables|Default|GetBlackboard) (Utilities|Name|MakeLiteralName "targetActor") (Utilities|SelectObject (Game|GetPlayerCharacter 0) 0 (.bsuccessfullysensed stimulus)))
      (if (not (.bsuccessfullysensed stimulus))
        (AI|Components|Blackboard|SetValueasVector (Variables|Default|GetBlackboard) (Utilities|Name|MakeLiteralName "lastKnownLocation") (.stimuluslocation stimulus))))))