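; BP_BasicEnemy is a basic enemy actor that flashes red when it is hit.
; The construction script makes a dynamic material instance on the Cylinder mesh.
; Tick polls the IsHit flag, clears it, sets the material's color parameter to red, and resets it to white after a one-second delay.
; Nothing in this graph sets IsHit.
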(event Custom|GotHit
  (Rendering|Material|SetVectorParameterValue (Variables|Default|Getmaterial) "color" "(R=1.000000,G=0.000000,B=0.074020,A=1.000000)" :!class /Script/Engine.MaterialInstanceDynamic))

(event Custom|ResetColor
  (Rendering|Material|SetVectorParameterValue (Variables|Default|Getmaterial) "color" "(R=1.000000,G=1.000000,B=1.000000,A=1.000000)" :!class /Script/Engine.MaterialInstanceDynamic))

(event EventBeginPlay)

(event Collision|EventActorBeginOverlap
  (params (OtherActor :type Actor%20Object%20Reference)))

(event EventTick
  (params (DeltaSeconds :type Float%20%28single-precision%29))
  (if (Variables|Default|GetisHit)
    (Variables|Default|SetisHit false)
    (CallFunction|GotHit)
    (Utilities|FlowControl|Delay 1.0)
    (CallFunction|ResetColor)))

(fn ConstructionScript
  (bind _cylinder (Variables|Default|GetCylinder))
  (bind _returnvalue (Rendering|Material|CreateDynamicMaterialInstance _cylinder 0 (Rendering|Material|GetMaterial _cylinder 0) "None" :!class /Script/Engine.PrimitiveComponent))
  (Variables|Default|Setmaterial _returnvalue))